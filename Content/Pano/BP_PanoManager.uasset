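; BP_PanoManager displays panorama textures on a sphere and switches between them by movement direction.
; BeginPlay wraps the sphere's material in a dynamic instance.
; SetPanoTexture looks up an index in a direction-to-index map, range-checks it against the texture array and updates the PanoTexture parameter.
; A helper converts a 2D input action value into a direction enum using the signs of its truncated axes.
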(event `self.ReceiveBeginPlay`
  ; BEGINPLAY - CREATE DYNAMIC MI AND INITIALIZE SPHERE TO DEFAULT CENTER MATERIAL
  (`KismetSystemLibrary.PrintString` "In pano manager")
  (bind _returnvalue (`KismetMaterialLibrary.CreateDynamicMaterialInstance` (`PrimitiveComponent.GetMaterial` (`self.Sphere`) 0) "DML_Sphere"))
  (bind _output_get (set `self.DynamicMat` _returnvalue))
  (`PrimitiveComponent.SetMaterial` (`self.Sphere`) 0 _output_get))

(event `Set Pano Texture`
  (params (`Movement Direction` :type "/Game/Pano/E_PanoramaDirection Enum" :default "NewEnumerator0"))
  (bind _dynamicmat (`self.DynamicMat`))
  ; SET PANO TEXTURE - GIVEN A TEXTURE INDEX (THAT INDICATES DIRECTION), UPDATE THE DYNAMIC MATERIAL
  (`KismetSystemLibrary.PrintString` "Setting Pano Texture")
  (bind _new_pano_index (`self.UpdatePanoIndex` `Movement Direction`))
  (if (< _new_pano_index (`KismetArrayLibrary.Array_Length` (`self.PanoramaTextures`)))
    (`KismetSystemLibrary.PrintString` (`KismetSystemLibrary.GetDisplayName` _dynamicmat))
    (`MaterialInstanceDynamic.SetTextureParameterValue` _dynamicmat "PanoTexture" (`|GetArrayItem` (`self.PanoramaTextures`) (`self.CurrentPanoramaIndex`)))
    (`KismetSystemLibrary.PrintString` (`KismetSystemLibrary.GetDisplayName` (`self.DynamicMat`)))
    (else
      (`KismetSystemLibrary.PrintString` "Invalid texture index!"))))

(fn `Convert Action Value to E_PanoDirection`
  (params (`Action Value` :type "Vector2D Structure"))
  (returns (`Direction Enum` :type "/Game/Pano/E_PanoramaDirection Enum"))
  (bind (_x _y) (`KismetMathLibrary.BreakVector2D` `Action Value`))
  (`KismetSystemLibrary.PrintString` "Converting Action Value")
  (switch `int` (+ (* (`KismetMathLibrary.SignOfInteger` (`KismetMathLibrary.FTrunc` _x)) 3) (`KismetMathLibrary.SignOfInteger` (`KismetMathLibrary.FTrunc` _y)))
    (:`Default`
      (set `self.CurrentMovementDirection` "NewEnumerator0" :!label _label))
    (:`-3`
      (set `self.CurrentMovementDirection` "NewEnumerator2"))
    (:`-1`
      (set `self.CurrentMovementDirection` "NewEnumerator2"))
    (:`0`
      (goto _label))
    (:`1`
      (set `self.CurrentMovementDirection` "NewEnumerator1"))
    (:`3`
      (set `self.CurrentMovementDirection` "NewEnumerator4")))
  (return (`self.CurrentMovementDirection`)))

(fn `UpdatePanoIndex`
  (params (`Movement Direction` :type "/Game/Pano/E_PanoramaDirection Enum" :default "NewEnumerator0"))
  (returns (`New Pano Index` :type Integer))
  (bind (_value _returnvalue) (`BlueprintMapLibrary.Map_Find` (`self.DirectionToIndexMap`) `Movement Direction`))
  (if (`KismetMathLibrary.Conv_IntToBool` _value)
    (bind _output_get (set `self.CurrentPanoramaIndex` _value))
    (return _output_get)
    (else
      (`KismetSystemLibrary.PrintString` "Invalid movement direction" _returnvalue))))

(fn `UserConstructionScript`)