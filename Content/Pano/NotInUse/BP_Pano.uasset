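; Panorama actor that displays a material on its Sphere mesh, kept in a NotInUse folder.
; BeginPlay creates a dynamic instance of CenterMaterial, stores it as DynamicMaterial and applies it to the sphere.
; UpdatePanoMaterial ignores its NewTexture input and writes EmissiveColor to "PanoramaTexture" as a vector parameter.
; The newPano event is empty, and the logic to swap in a new material instance is disconnected.
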(event `self.ReceiveBeginPlay`
  (bind _returnvalue (`KismetMaterialLibrary.CreateDynamicMaterialInstance` (`self.centerMaterial`)))
  (set `self.DynamicMaterial` _returnvalue)
  (`PrimitiveComponent.SetMaterial` (`self.Sphere`) 0 (`self.DynamicMaterial`)))

(event `newPano`
  (params (NewMI :type "MaterialInstance Object Reference")))

(event `UpdatePanoMaterial`
  (params (NewTexture :type "Material Object Reference"))
  (`MaterialInstanceDynamic.SetVectorParameterValue` (`self.DynamicMaterial`) "PanoramaTexture" (`self.EmissiveColor`)))

(fn `UserConstructionScript`)